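; Player gameplay ability that toggles lock-on to the closest enemy found around the avatar.
; It queries and sets the target through message calls on the avatar: an existing target is cleared, otherwise the closest enemy becomes the target.
; When no enemy character is found, it also clears the target.
; The target's LockIcon is shown or hidden to match, and a short WaitDelay precedes EndAbility after each change.
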(event `self.K2_ActivateAbility`
  (bind _returnvalue (`self.GetAvatarActorFromActorInfo`))
  (bind _returnvalue_2 (`self.GetAvatarActorFromActorInfo`))
  (bind _returnvalue_3 (message `CombatInterface.GetClosestEnemy` (`self.GetAvatarActorFromActorInfo`) 300.0 2000.0))
  (bind _asslcharacter_base (cast `SLCharacterBase` _returnvalue_3)
    (:`then`
      (`/Engine/EditorBlueprintResources/StandardMacros.IsValid` _asslcharacter_base
        (:`Is Valid`
          (bind _returnvalue_4 (message `CombatInterface.GetLockOnTarget` (`self.GetAvatarActorFromActorInfo`)))
          (if (`KismetSystemLibrary.IsValid` _returnvalue_4)
            (bind _returnvalue_5 (message `CombatInterface.GetLockOnTarget` _returnvalue_2 :!label _label))
            (bind _asbp_enemy_character_base (cast `/Game/BluePrint/Character/Enemy/BP_EnemyCharacterBase` _returnvalue_5)
              (:`then`
                (`SceneComponent.SetVisibility` (`/Game/BluePrint/Character/Enemy/BP_EnemyCharacterBase.LockIcon` _asbp_enemy_character_base) false false))
              (:`CastFailed`
                _))
            (message `CombatInterface.SetLockOnTarget` _returnvalue_2 null)
            (`AbilityTask_WaitDelay.WaitDelay` 1.0
              (:`OnFinish`
                (`self.K2_EndAbility`)))
            (else
              (message `CombatInterface.SetLockOnTarget` _returnvalue _asslcharacter_base)
              (bind _returnvalue_6 (message `CombatInterface.GetLockOnTarget` _returnvalue))
              (bind _asbp_enemy_character_base_2 (cast `/Game/BluePrint/Character/Enemy/BP_EnemyCharacterBase` _returnvalue_6)
                (:`then`
                  (`SceneComponent.SetVisibility` (`/Game/BluePrint/Character/Enemy/BP_EnemyCharacterBase.LockIcon` _asbp_enemy_character_base_2) true false))
                (:`CastFailed`
                  _))
              (`AbilityTask_WaitDelay.WaitDelay` 1.0
                (:`OnFinish`
                  (`self.K2_EndAbility`))))))
        (:`Is Not Valid`
          (`self.K2_EndAbility`))))
    (:`CastFailed`
      (goto _label))))