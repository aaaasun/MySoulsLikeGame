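; Player heavy attack gameplay ability that plays a combo montage chosen by the avatar's combo code.
; On activation it commits, sets the damage effect spec and plays the indexed montage.
; After a delay it listens for a Combo.LightAttack event to increment the code, alongside a short timed reset to zero.
; On ability end, a code past the last montage wraps to zero.
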(event `self.K2_ActivateAbility`
  (bind _returnvalue (`self.GetAvatarActorFromActorInfo`))
  (`self.K2_CommitAbility`)
  (`self.SetDamageEffectSpecHandle`)
  (bind _returnvalue_2 (`self.GetAttackMontages`))
  (bind _returnvalue_3 (message `CombatInterface.GetComboCode` (`self.GetAvatarActorFromActorInfo`)))
  (bind _output_get (set `self.TaggedMontage` (`|GetArrayItem` _returnvalue_2 _returnvalue_3)))
  (bind _montage (break `TaggedMontage` _output_get))
  (`/Engine/EditorBlueprintResources/StandardMacros.IsValid` _montage
    (:`Is Valid`
      (`AbilityTask_PlayMontageAndWait.CreatePlayMontageAndWaitProxy` "None" _montage 1.0 "None" false
        (:`then`
          (`AbilityTask_WaitDelay.WaitDelay` 1.5
            (:`OnFinish`
              (`AbilityTask_WaitGameplayEvent.WaitGameplayEvent` (struct :`TagName` "Combo.LightAttack") null
                (:`then`
                  (`KismetSystemLibrary.Delay` 0.5)
                  (message `CombatInterface.SetComboCode` _returnvalue 0))
                (:`EventReceived`
                  (bind _returnvalue_4 (message `CombatInterface.GetComboCode` _returnvalue))
                  (bind _result (`/Engine/EditorBlueprintResources/StandardMacros.IncrementInt` _returnvalue_4)
                    (:`  `
                      (message `CombatInterface.SetComboCode` (`self.GetAvatarActorFromActorInfo`) _result)))))
              (`self.K2_EndAbility`))))
        (:`OnCompleted`
          (`self.K2_EndAbility`))))))

(event `self.K2_OnEndAbility`
  (params (bWasCancelled :type Boolean))
  (bind _returnvalue (`self.GetAttackMontages`))
  (bind _returnvalue_2 (message `CombatInterface.GetComboCode` (`self.GetAvatarActorFromActorInfo`)))
  (if (>= _returnvalue_2 (`KismetArrayLibrary.Array_Length` _returnvalue))
    (message `CombatInterface.SetComboCode` (`self.GetAvatarActorFromActorInfo`) 0)))