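; Player Gameplay Ability that plays a hit reaction while stopping the avatar's movement.
; On activation it zeroes max walk speed, applies GE_HitReact to the owner, and plays the montage supplied by the avatar's CombatInterface.
; When the montage completes, is interrupted or is cancelled, it removes the effect by its stored handle and ends.
; OnEndAbility sets walk speed back to a hardcoded value rather than the previous one.
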(event `self.K2_ActivateAbility`
  (set `CharacterMovementComponent.MaxWalkSpeed` 0.0 (`Actor.GetComponentByClass` (`self.GetAvatarActorFromActorInfo`) "/Script/Engine.CharacterMovementComponent"))
  (bind _returnvalue (`self.BP_ApplyGameplayEffectToOwner` "/Game/BluePrint/AbilitySystem/GameplayEffects/Enemy/GE_HitReact.GE_HitReact_C"))
  (set `self.Active GE HitReact` _returnvalue)
  (bind _ascombat_interface (cast `CombatInterface` (`self.GetAvatarActorFromActorInfo`)))
  (bind _returnvalue_2 (`CombatInterface.GetHitReactMontage` _ascombat_interface))
  (`AbilityTask_PlayMontageAndWait.CreatePlayMontageAndWaitProxy` "None" _returnvalue_2
    (:`OnCompleted`
      _)
    (:`OnInterrupted`
      _)
    (:`OnCancelled`
      _))
  (`self.BP_RemoveGameplayEffectFromOwnerWithHandle` (`self.Active GE HitReact`))
  (`self.K2_EndAbility`))

(event `self.K2_OnEndAbility`
  (params (bWasCancelled :type Boolean))
  (set `CharacterMovementComponent.MaxWalkSpeed` 600.0 (`Actor.GetComponentByClass` (`self.GetAvatarActorFromActorInfo`) "/Script/Engine.CharacterMovementComponent")))