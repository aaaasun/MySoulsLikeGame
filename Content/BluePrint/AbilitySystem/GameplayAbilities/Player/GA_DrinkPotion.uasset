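; Player gameplay ability that drinks a healing potion, rooting the avatar in place while it does.
; Activation commits the ability, sets MaxWalkSpeed to zero and plays the drink montage.
; The montage's PotionHeal gameplay event applies GE_PotionHealth to the owner once, timing the heal to the animation.
; Any montage exit ends the ability, and OnEndAbility sets walk speed to a hardcoded value rather than restoring the previous one.
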(event `self.K2_ActivateAbility`
  (`self.K2_CommitAbility`)
  (set `CharacterMovementComponent.MaxWalkSpeed` 0.0 (`Actor.GetComponentByClass` (`self.GetAvatarActorFromActorInfo`) "/Script/Engine.CharacterMovementComponent"))
  (`AbilityTask_PlayMontageAndWait.CreatePlayMontageAndWaitProxy` "None" "/Game/BluePrint/Montage/Player/MA_DrinkPotion.MA_DrinkPotion" 1.0 "None" false
    (:`then`
      (`AbilityTask_WaitGameplayEvent.WaitGameplayEvent` (struct :`TagName` "Event.Montage.PotionHeal") null true
        (:`EventReceived`
          (`self.BP_ApplyGameplayEffectToOwner` "/Game/BluePrint/Actor/Potion/GE_PotionHealth.GE_PotionHealth_C"))))
    (:`OnCompleted`
      (`self.K2_EndAbility` :!label _label))
    (:`OnBlendOut`
      (goto _label))
    (:`OnInterrupted`
      (goto _label))
    (:`OnCancelled`
      (goto _label))))

(event `self.K2_OnEndAbility`
  (params (bWasCancelled :type Boolean))
  (set `CharacterMovementComponent.MaxWalkSpeed` 600.0 (`Actor.GetComponentByClass` (`self.GetAvatarActorFromActorInfo`) "/Script/Engine.CharacterMovementComponent")))