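; GA_Pickup is a player gameplay ability that picks up the weapon the avatar is overlapping.
; On activation it fetches the avatar's combat component and, only on the authority, the overlapped weapon through message calls.
; When both are valid, the combat component equips the weapon and adds that weapon's abilities.
; Every path ends the ability immediately.
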(event `self.K2_ActivateAbility`
  (bind _returnvalue (`self.GetAvatarActorFromActorInfo`))
  (bind _returnvalue_2 (message `CombatInterface.GetCombatComponent` _returnvalue))
  (`/Engine/EditorBlueprintResources/StandardMacros.IsValid` _returnvalue_2
    (:`Is Valid`
      (if (`Actor.HasAuthority` _returnvalue)
        (bind _returnvalue_3 (message `CombatInterface.GetOverlapWeapon` (`self.GetAvatarActorFromActorInfo`)))
        (`/Engine/EditorBlueprintResources/StandardMacros.IsValid` _returnvalue_3
          (:`Is Valid`
            (`CombatComponent.EquipWeapon` _returnvalue_2 _returnvalue_3)
            (`CombatComponent.AddWeaponAbilities` _returnvalue_2 _returnvalue_3)
            (`self.K2_EndAbility`))
          (:`Is Not Valid`
            (`self.K2_EndAbility`)))
        (else
          (`self.K2_EndAbility`))))
    (:`Is Not Valid`
      (`self.K2_EndAbility`))))