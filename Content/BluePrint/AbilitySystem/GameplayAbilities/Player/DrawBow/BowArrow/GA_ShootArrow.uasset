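; Player bow gameplay ability that fires an arrow at a targeted impact point.
; On activation it commits, takes the impact point from hit-result target data and plays the first attack montage at increased rate.
; A fire-arrow montage event spawns the projectile and starts the draw-arrow montage.
; The ability ends when the attack montage completes or the draw montage finishes or is interrupted, without stopping either montage.
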(event `self.K2_ActivateAbility`
  (`self.K2_CommitAbility`)
  (bind (_asynctaskproxy _datahandle) (`HitResultTargetData.CreateHitResultTargetData`)
    (:`ValidData`
      (set `self.ProjectileImpactPoint` (`.ImpactPoint` (`GameplayStatics.BreakHitResult` (`AbilitySystemBlueprintLibrary.GetHitResultFromTargetData` _datahandle))))
      (bind _returnvalue (`self.GetAttackMontages`))
      (bind _output_get (set `self.TaggedMontages` (`|GetArrayItem` _returnvalue)))
      (`AbilityTask_PlayMontageAndWait.CreatePlayMontageAndWaitProxy` "None" (`.Montage` (break `TaggedMontage` _output_get)) 2.0 "None" false
        (:`then`
          (`AbilityTask_WaitGameplayEvent.WaitGameplayEvent` (struct :`TagName` "Event.Montage.FireBowArrow") null
            (:`EventReceived`
              (`self.SpawnProjectile` (`self.ProjectileImpactPoint`))
              (`AbilityTask_PlayMontageAndWait.CreatePlayMontageAndWaitProxy` "None" "/Game/BluePrint/Montage/Player/MA_DrawArrow.MA_DrawArrow" 1.0 "None" false
                (:`OnCompleted`
                  _)
                (:`OnBlendOut`
                  _)
                (:`OnInterrupted`
                  _)
                (:`OnCancelled`
                  _))
              (`self.K2_EndAbility`))))
        (:`OnCompleted`
          (`self.K2_EndAbility`))))))