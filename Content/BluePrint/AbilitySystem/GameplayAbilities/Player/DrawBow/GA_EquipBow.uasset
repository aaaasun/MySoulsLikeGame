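; Player gameplay ability that keeps the bow equipped while its input is held.
; On a successful commit, it sends an equip-bow message to the avatar and waits for input release to end the ability.
; Ending sends an unload-bow message to the avatar.
; The crosshair widget is created and removed only without authority, so a listen-server host does not get one from this ability.
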(event `self.K2_ActivateAbility`
  (bind _returnvalue (`self.K2_CommitAbility`))
  (if _returnvalue
    (message `/Game/BluePrint/Interface/BPI_Weapon.EquipBow` (`self.GetAvatarActorFromActorInfo`))
    (`self.K2_HasAuthority`
      (:`True`
        _)
      (:`False`
        (bind _returnvalue_2 (`|CreateWidget` "/Game/BluePrint/UI/Crosshairs/WBP_Crosshairs.WBP_Crosshairs_C"))
        (bind _output_get (set `self.CrosshairsWidget` _returnvalue_2))
        (`UserWidget.AddToViewport` _output_get 0)))
    (`AbilityTask_WaitInputRelease.WaitInputRelease` false
      (:`OnRelease`
        (`self.K2_EndAbility`)))
    (else
      (`self.K2_EndAbility`))))

(event `self.K2_OnEndAbility`
  (params (bWasCancelled :type Boolean))
  (message `/Game/BluePrint/Interface/BPI_Weapon.UnloadBow` (`self.GetAvatarActorFromActorInfo`))
  (`self.K2_HasAuthority`
    (:`False`
      (`Widget.RemoveFromParent` (`self.CrosshairsWidget`)))))