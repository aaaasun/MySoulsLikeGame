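; Player light-attack gameplay ability that plays a melee montage and damages enemies it hits.
; It plays the first tagged montage from GetAttackMontages and listens for that montage's gameplay event tag.
; Each event finds live players between two hit-scan sockets on the tag's combat component and applies damage to non-friendly ones.
; The ability ends when the montage completes, blends out, or is interrupted or cancelled.
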(event `self.K2_ActivateAbility`
  (bind _returnvalue (`self.GetAvatarActorFromActorInfo`))
  (bind _returnvalue_2 (`self.GetAttackMontages`))
  (bind _output_get (set `self.TaggedMontage` (`|GetArrayItem` _returnvalue_2)))
  (bind (_montage _montagetag) (break `TaggedMontage` _output_get))
  (`/Engine/EditorBlueprintResources/StandardMacros.IsValid` _montage
    (:`Is Valid`
      (`AbilityTask_PlayMontageAndWait.CreatePlayMontageAndWaitProxy` "None" _montage 1.0 "None" false
        (:`then`
          (`AbilityTask_WaitGameplayEvent.WaitGameplayEvent` _montagetag null
            (:`EventReceived`
              (bind _returnvalue_3 (message `CombatInterface.GetCombatComponent` _returnvalue _montagetag))
              (bind _outoverlappingactors (`SLAbilitySystemBlueprintLibrary.GetLivePlayersWithinRadius` _returnvalue (`|MakeArray` _returnvalue) (`self.Extent`) (`SceneComponent.GetSocketLocation` _returnvalue_3 "HitScanSocket1") (`SceneComponent.GetSocketLocation` _returnvalue_3 "HitScanSocket2")))
              (for _array_element _outoverlappingactors
                (if (`SLAbilitySystemBlueprintLibrary.IsNotFriend` (`self.GetAvatarActorFromActorInfo`) _array_element)
                  (`self.CauseDamage` _array_element))))))
        (:`OnCompleted`
          (`self.K2_EndAbility` :!label _label))
        (:`OnBlendOut`
          (goto _label))
        (:`OnInterrupted`
          (goto _label))
        (:`OnCancelled`
          (goto _label))))))

(event `self.K2_OnEndAbility`
  (params (bWasCancelled :type Boolean)))