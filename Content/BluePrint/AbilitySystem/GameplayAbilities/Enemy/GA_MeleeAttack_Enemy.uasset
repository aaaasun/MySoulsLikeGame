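; Enemy melee attack gameplay ability that turns the avatar toward its combat target and plays a random attack montage.
; On activation it sets the damage effect spec, updates facing through CombatInterface, picks a tagged montage and ends when the montage completes, blends out or is interrupted or cancelled.
; A montage-event hit scan between two sockets that damages non-friendly live players is present but unconnected, so this graph applies no damage itself.
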(event `self.K2_ActivateAbility`
  (bind _returnvalue (`self.GetAvatarActorFromActorInfo`))
  (`self.SetDamageEffectSpecHandle`)
  (bind _returnvalue_2 (message `EnemyInterface.GetCombatTarget` _returnvalue))
  (bind _ascombat_interface (cast `CombatInterface` _returnvalue))
  (`CombatInterface.UpdateFacingTarget` _ascombat_interface (`Actor.K2_GetActorLocation` _returnvalue_2))
  (bind _returnvalue_3 (`self.GetAttackMontages`))
  (bind _output_get (set `self.TaggedMontage` (`self.GetRandomTaggedMontageFromArray` _returnvalue_3)))
  (`AbilityTask_PlayMontageAndWait.CreatePlayMontageAndWaitProxy` "None" (`.Montage` (break `TaggedMontage` _output_get)) 1.0 "None" false
    (:`OnCompleted`
      _)
    (:`OnBlendOut`
      _)
    (:`OnInterrupted`
      _)
    (:`OnCancelled`
      _))
  (`self.K2_EndAbility`))