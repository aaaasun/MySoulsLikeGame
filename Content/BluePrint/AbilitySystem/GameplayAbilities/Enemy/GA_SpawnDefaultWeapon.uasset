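; Enemy gameplay ability that equips the avatar's default weapon when activated.
; On the authority only, it gets the combat component and looks up a melee weapon by tag, falling back to a ranged one.
; The found weapon is equipped and its abilities are added through the combat component, and the ability ends on every path.
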(event `self.K2_ActivateAbility`
  (bind _returnvalue (`self.GetAvatarActorFromActorInfo`))
  (bind _returnvalue_2 (`self.GetAvatarActorFromActorInfo`))
  (bind _returnvalue_3 (message `CombatInterface.GetCombatComponent` _returnvalue))
  (`/Engine/EditorBlueprintResources/StandardMacros.IsValid` _returnvalue_3
    (:`Is Valid`
      (if (`Actor.HasAuthority` _returnvalue)
        (bind _returnvalue_4 (message `CombatInterface.GetCombatWeapon` _returnvalue_2 (`self.MeleeWeaponTag`)))
        (`/Engine/EditorBlueprintResources/StandardMacros.IsValid` _returnvalue_4
          (:`Is Valid`
            (`CombatComponent.EquipWeapon` _returnvalue_3 _returnvalue_4)
            (`CombatComponent.AddWeaponAbilities` _returnvalue_3 _returnvalue_4)
            (`self.K2_EndAbility`))
          (:`Is Not Valid`
            (bind _returnvalue_5 (message `CombatInterface.GetCombatWeapon` _returnvalue_2 (`self.RangedWeaponTag`)))
            (`/Engine/EditorBlueprintResources/StandardMacros.IsValid` _returnvalue_5
              (:`Is Valid`
                (`CombatComponent.EquipWeapon` _returnvalue_3 _returnvalue_5)
                (`CombatComponent.AddWeaponAbilities` _returnvalue_3 _returnvalue_5)
                (`self.K2_EndAbility`))
              (:`Is Not Valid`
                (`self.K2_EndAbility`)))))
        (else
          (`self.K2_EndAbility`))))
    (:`Is Not Valid`
      (`self.K2_EndAbility`))))