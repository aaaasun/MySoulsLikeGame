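; GA_ShootArrow is a Gameplay Ability that fires an arrow from a bow.
; After committing, it gets the impact point from a hit-result target data task and plays the fire montage at increased rate.
; The Event.Montage.FireBowArrow gameplay event times SpawnProjectile toward that point, then starts the draw-arrow montage.
; The ability ends when that montage completes, blends out or is interrupted or cancelled, or when the commit fails.
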(event `self.K2_ActivateAbility`
  (bind _returnvalue (`self.K2_CommitAbility`))
  (if _returnvalue
    (bind (_asynctaskproxy _datahandle) (`HitResultTargetData.CreateHitResultTargetData`)
      (:`ValidData`
        (set `self.ProjectileImpactPoint` (`.ImpactPoint` (`GameplayStatics.BreakHitResult` (`AbilitySystemBlueprintLibrary.GetHitResultFromTargetData` _datahandle))))
        (`AbilityTask_PlayMontageAndWait.CreatePlayMontageAndWaitProxy` "None" "/Game/BluePrint/Montage/Player/MA_FireArrow.MA_FireArrow" 2.0
          (:`then`
            (`AbilityTask_WaitGameplayEvent.WaitGameplayEvent` (struct :`TagName` "Event.Montage.FireBowArrow") null
              (:`EventReceived`
                (`self.SpawnProjectile` (`self.ProjectileImpactPoint`))
                (`AbilityTask_PlayMontageAndWait.CreatePlayMontageAndWaitProxy` "None" "/Game/BluePrint/Montage/Player/MA_DrawArrow.MA_DrawArrow"
                  (:`OnCompleted`
                    _)
                  (:`OnBlendOut`
                    _)
                  (:`OnInterrupted`
                    _)
                  (:`OnCancelled`
                    _)))))))))
  (`self.K2_EndAbility`))