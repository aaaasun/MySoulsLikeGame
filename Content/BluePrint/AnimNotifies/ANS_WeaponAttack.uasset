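; Anim notify state that marks the active attack window of a weapon during an animation, for player and enemy characters.
; It checks the mesh owner for the "Player" tag, then casts to BP_PlayerCharacter or BP_EnemyCharacterBase.
; The character resolves a combat weapon from MontageTag, which receives BeginWeaponAttack when the notify starts and EndWeaponAttack when it ends.
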(fn `Received_NotifyBegin`
  (params (MeshComp :type "SkeletalMeshComponent Object Reference") (Animation :type "AnimSequenceBase Object Reference") (TotalDuration :type "Float (single-precision)") (EventReference :type "AnimNotifyEventReference Structure (by ref)"))
  (returns (ReturnValue :type Boolean))
  (bind _returnvalue (`ActorComponent.GetOwner` MeshComp))
  (if (`Actor.ActorHasTag` _returnvalue "Player")
    (bind _asbp_player_character (cast `/Game/BluePrint/Character/Player/BP_PlayerCharacter` _returnvalue))
    (`/Engine/EditorBlueprintResources/StandardMacros.IsValid` _asbp_player_character
      (:`Is Valid`
        (bind _returnvalue_2 (message `CombatInterface.GetCombatWeapon` _asbp_player_character (`self.Montage Tag`)))
        (`/Engine/EditorBlueprintResources/StandardMacros.IsValid` _returnvalue_2
          (:`Is Valid`
            (`SLBaseWeapon.BeginWeaponAttack` _returnvalue_2)
            (return false)))))
    (else
      (bind _asbp_enemy_character_base (cast `/Game/BluePrint/Character/Enemy/BP_EnemyCharacterBase` _returnvalue))
      (`/Engine/EditorBlueprintResources/StandardMacros.IsValid` _asbp_enemy_character_base
        (:`Is Valid`
          (bind _returnvalue_3 (message `CombatInterface.GetCombatWeapon` _asbp_enemy_character_base (`self.Montage Tag`)))
          (`/Engine/EditorBlueprintResources/StandardMacros.IsValid` _returnvalue_3
            (:`Is Valid`
              (`SLBaseWeapon.BeginWeaponAttack` _returnvalue_3)
              (return false))))))))

(fn `Received_NotifyEnd`
  (params (MeshComp :type "SkeletalMeshComponent Object Reference") (Animation :type "AnimSequenceBase Object Reference") (EventReference :type "AnimNotifyEventReference Structure (by ref)"))
  (returns (ReturnValue :type Boolean))
  (bind _returnvalue (`ActorComponent.GetOwner` MeshComp))
  (if (`Actor.ActorHasTag` _returnvalue "Player")
    (bind _asbp_player_character (cast `/Game/BluePrint/Character/Player/BP_PlayerCharacter` _returnvalue))
    (`/Engine/EditorBlueprintResources/StandardMacros.IsValid` _asbp_player_character
      (:`Is Valid`
        (bind _returnvalue_2 (message `CombatInterface.GetCombatWeapon` _asbp_player_character (`self.Montage Tag`)))
        (`/Engine/EditorBlueprintResources/StandardMacros.IsValid` _returnvalue_2
          (:`Is Valid`
            (`SLBaseWeapon.EndWeaponAttack` _returnvalue_2)
            (return false)))))
    (else
      (bind _asbp_enemy_character_base (cast `/Game/BluePrint/Character/Enemy/BP_EnemyCharacterBase` _returnvalue))
      (`/Engine/EditorBlueprintResources/StandardMacros.IsValid` _asbp_enemy_character_base
        (:`Is Valid`
          (bind _returnvalue_3 (message `CombatInterface.GetCombatWeapon` _asbp_enemy_character_base (`self.Montage Tag`)))
          (`/Engine/EditorBlueprintResources/StandardMacros.IsValid` _returnvalue_3
            (:`Is Valid`
              (`SLBaseWeapon.EndWeaponAttack` _returnvalue_3)
              (return false))))))))