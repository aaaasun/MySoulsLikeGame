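; Player controller Blueprint that opens and closes the attribute menu when the IA_Setup input action starts.
; OpenAndCloseMenu toggles on an IsMenuOpen flag, creating a new WBP_AttributeMenu widget on each open and removing it from the viewport on close.
; Opening also switches to Game and UI input focused on the widget, shows the cursor and pauses the game, while closing reverts all three.
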(event `EnhancedInput|/Game/BluePrint/Input/InputActions/IA_Setup`
  (params (ActionValue :type Boolean) (ElapsedSeconds :type "Float (double-precision)") (TriggeredSeconds :type "Float (double-precision)") (InputAction :type "InputAction Object Reference" :default "/Game/BluePrint/Input/InputActions/IA_Setup.IA_Setup"))
  (:`Started`
    (`self.OpenAndCloseMenu`)))

(fn `OpenAndCloseMenu`
  (if (not (`self.IsMenuOpen?`))
    (set `self.IsMenuOpen?` true)
    (bind _returnvalue (`|CreateWidget` "/Game/BluePrint/UI/AttributeMenu/WBP_AttributeMenu.WBP_AttributeMenu_C" self))
    (bind _output_get (set `self.BP_AttributeMenuWidget` _returnvalue))
    (`UserWidget.AddToViewport` _output_get 0)
    (`WidgetBlueprintLibrary.SetInputMode_GameAndUIEx` self (`self.BP_AttributeMenuWidget`))
    (set `self.bShowMouseCursor` true)
    (`GameplayStatics.SetGamePaused` true)
    (else
      (set `self.IsMenuOpen?` false)
      (`Widget.RemoveFromParent` (`self.BP_AttributeMenuWidget`))
      (`WidgetBlueprintLibrary.SetInputMode_GameOnly` self)
      (set `self.bShowMouseCursor` false)
      (`GameplayStatics.SetGamePaused` false))))

(fn `UserConstructionScript`)