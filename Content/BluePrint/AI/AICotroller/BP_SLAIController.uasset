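; AI controller that uses AI Perception to pick a living Player-tagged actor as its target and feed the Blackboard.
; Perception updates read each living actor's first stimulus, setting or clearing TargetToFollow and toggling the pawn's staring state via interface message.
; Tick clears a dead target, otherwise writes the pawn's distance to the last sensed actor into DistanceToTarget.
; A per-stimulus loop and switch remain unconnected.
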(event `self.ReceiveTick`
  (params (DeltaSeconds :type "Float (single-precision)"))
  (bind _returnvalue (`BlackboardComponent.GetValueAsObject` (`self.Blackboard`) "TargetToFollow"))
  (`/Engine/EditorBlueprintResources/StandardMacros.IsValid` _returnvalue
    (:`Is Valid`
      (bind _returnvalue_2 (message `CombatInterface.IsDead` _returnvalue))
      (if _returnvalue_2
        (`BlackboardComponent.SetValueAsObject` (`self.Blackboard`) "TargetToFollow" null)
        (else
          (`BlackboardComponent.SetValueAsFloat` (`self.Blackboard`) "DistanceToTarget" (`self.GetDistanceTo` (`self.K2_GetPawn`) (`self.SensedActor`))))))))

(event `self.AIPerception.OnPerceptionUpdated`
  (params (UpdatedActors :type "Array of Actor Object Reference (by ref)"))
  (`self.UpdatePerception` UpdatedActors))

(fn `UpdatePerception`
  (params (PerceivedActors :type "Array of Actor Object Reference"))
  (locals (L_SensedActor :type "Actor Object Reference") (L_AIStimilus :type "AIStimulus Structure"))
  (for _array_element PerceivedActors
    (bind _returnvalue (message `CombatInterface.IsDead` _array_element))
    (if (not _returnvalue)
      (set `self.SensedActor` _array_element)
      (bind _info (`AIPerceptionComponent.GetActorsPerception` (`self.AIPerception`) (`self.SensedActor`)))
      (set `local.L_AIStimilus` (`|GetArrayItem` (`.LastSensedStimuli` (break `ActorPerceptionBlueprintInfo` _info))))
      (if (`.bSuccessfullySensed` (break `AIStimulus` (`local.L_AIStimilus`)))
        (if (`self.ActorHasTag` (`self.SensedActor`) "Player")
          (`BlackboardComponent.SetValueAsObject` (`self.Blackboard`) "TargetToFollow" (`self.SensedActor`))
          (message `CombatInterface.SetbIsStaring` (`self.K2_GetPawn`) true))
        (else
          (`BlackboardComponent.SetValueAsObject` (`self.Blackboard`) "TargetToFollow" null)
          (`BlackboardComponent.SetValueAsFloat` (`self.Blackboard`) "DistanceToTarget" 0.0)
          (message `CombatInterface.SetbIsStaring` (`self.K2_GetPawn`) false))))))

(fn `UserConstructionScript`)