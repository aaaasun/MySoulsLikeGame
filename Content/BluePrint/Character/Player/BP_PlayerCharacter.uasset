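; Player character Blueprint that handles bow equip and unequip and overrides the ability combo event.
; Equipping and unloading play montages, toggle the aim flag, and switch rotation between controller yaw while aiming and movement direction otherwise.
; The first equip also grants character abilities through a DoOnce.
; Combos jump to a random montage section from the ANSJumpSection list when that reference is valid.
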(event `self.ReceiveBeginPlay`)

(event `/Game/BluePrint/Interface/BPI_Weapon.EquipBow`
  ;[1 1 1] 装备弓
  (`self.PlayAnimMontage` "/Game/BluePrint/Montage/Player/MA_DrawArrow.MA_DrawArrow")
  (set `self.IsBowAim` true)
  (set `CharacterMovementComponent.bOrientRotationToMovement` false (`self.CharacterMovement`))
  (set `self.bUseControllerRotationYaw` true)
  (`/Engine/EditorBlueprintResources/StandardMacros.DoOnce` false
    (:`Completed`
      (`self.AddCharacterAbilities` (`self.In Abilities`)))))

(event `/Game/BluePrint/Interface/BPI_Weapon.UnloadBow`
  ;[1 1 1] 卸下弓
  (set `self.IsBowAim` false)
  (`self.PlayAnimMontage` "/Game/BluePrint/Montage/Player/MA_UnloadBow.MA_UnloadBow")
  (set `CharacterMovementComponent.bOrientRotationToMovement` true (`self.CharacterMovement`))
  (set `self.bUseControllerRotationYaw` false))

(event `CombatInterface.AbilitiesCombo`
  (bind _ans_jumpsection (`self.ANS_JumpSection`))
  (bind _jumpsections (`/Game/BluePrint/AnimNotifies/ANS_JumpSection.JumpSections` _ans_jumpsection))
  ;[1 1 1] 重写能力连击
  (`/Engine/EditorBlueprintResources/StandardMacros.IsValid` _ans_jumpsection
    (:`Is Valid`
      (`self.JumpSectionForCombo` (`|GetArrayItem` _jumpsections (`KismetMathLibrary.RandomInteger` (`KismetArrayLibrary.Array_Length` _jumpsections)))))))

(fn `UserConstructionScript`)